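; BP_Spike is a moving spike hazard that damages BP_Player on overlap with its Box.
; From BeginPlay, the MoveSpike timeline lerps the actor between CurrentLocation and TargetLocation, neither set in this graph.
; A Delay chained to the timeline's Update, rather than Finished, toggles IsDirectionChanged to replay or reverse the motion.
; Each overlap subtracts Health and opens PlatformerLevel at zero or below; an older lerp test remains unconnected.
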(event OnComponentBeginOverlap(Box)
  (params (OverlappedComponent :type Primitive%20Component%20Object%20Reference) (OtherActor :type Actor%20Object%20Reference) (OtherComp :type Primitive%20Component%20Object%20Reference) (OtherBodyIndex :type Integer) (bFromSweep :type Boolean) (SweepResult :type Hit%20Result%20Structure%20%28by%20ref%29))
  (bind _asbp_player (Utilities|Casting|CastToBP_Player OtherActor))
  (bind _output_get (Variables|/Game/Blueprints/BP_Player.BP_Player_C|SetHealth _asbp_player (- (Variables|/Game/Blueprints/BP_Player.BP_Player_C|GetHealth _asbp_player) 3e+01)))
  (if (<= _output_get 0.0)
    (Game|OpenLevel(byName) "PlatformerLevel")))

(event EventBeginPlay
  (bind _spikemove (Timeline|MoveSpike Play)
    (:Update
      (Transformation|SetActorLocation (Math|Vector|Lerp(Vector) (Variables|Default|GetCurrentLocation) (Variables|Default|GetTargetLocation) _spikemove) false false)
      (Utilities|FlowControl|Delay 1.0)
      (if (Variables|Default|GetisDirectionChanged)
        (Variables|Default|SetisDirectionChanged false)
        (Timeline|MoveSpike PlayFromStart)
        (else
          (Variables|Default|SetisDirectionChanged true)
          (Timeline|MoveSpike ReverseFromEnd))))))

(event Collision|EventActorBeginOverlap
  (params (OtherActor :type Actor%20Object%20Reference)))

(event EventTick
  (params (DeltaSeconds :type Float%20%28single-precision%29)))

(fn ConstructionScript)